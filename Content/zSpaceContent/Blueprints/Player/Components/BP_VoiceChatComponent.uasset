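; Voice chat component for the player that shows and hides the WBP_VoiceChat widget.
; On first show it async-loads the widget's soft class, creates it for player controller 0 and caches the reference for reuse.
; Showing adds the cached widget to the viewport and enables the mouse cursor; hiding removes it and disables the cursor.
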(event `HideVoiceChatWidget`
  (bind _voicechatwidgetref (`self.VoiceChatWidgetRef`)
    (:`then`
      (`Widget.RemoveFromParent` _voicechatwidgetref)
      (`self.ShowMouseCursor` false))
    (:`else`)))

(event `ShowVoiceChatWidget`
  (`self.VoiceChatWidgetRef`
    (:`then`
      (bind _voicechatwidgetref (`self.VoiceChatWidgetRef` :!label _label)
        (:`then`
          (if (not (`Widget.IsInViewport` _voicechatwidgetref))
            (`UserWidget.AddToViewport` _voicechatwidgetref (`self.ZOrder`))
            (`self.ShowMouseCursor` true)))
        (:`else`)))
    (:`else`
      (bind _class (`|LoadAssetClass` (`self.VoicChatWidgetSoftClassRef`))
        (:`Completed`
          (bind _aswbp_voice_chat (castclass `/Game/zSpaceContent/Blueprints/UMG/VoiceChat/WBP_VoiceChat` _class)
            (:`then`
              (bind _returnvalue (`|CreateWidget` _aswbp_voice_chat (`GameplayStatics.GetPlayerController` 0)))
              (set `self.VoiceChatWidgetRef` _returnvalue)
              (`KismetSystemLibrary.PrintString` "Info: Created Voic Chat Widget" true true (struct :`R` 0.252356 :`G` 1.0 :`A` 1.0))
              (goto _label))
            (:`CastFailed`
              (`KismetSystemLibrary.PrintString` "Error: The widget doesn't cast to WBP_VoiceChat"))))))))

(fn `ShowMouseCursor`
  (params (bShowMouseCursor :type Boolean))
  (set `PlayerController.bShowMouseCursor` bShowMouseCursor (`GameplayStatics.GetPlayerController` 0)))