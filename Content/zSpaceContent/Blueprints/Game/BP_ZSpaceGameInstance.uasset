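; BP_ZSpaceGameInstance is the game instance that controls the loading screen during play.
; RPG begin and end loading screen events show or hide a configurable loading widget through the widget loading manager object, with a high Z-order when shown.
; A separate HideLoadingDialog event also hides it, and all three skip the work on dedicated servers.
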(event `self.RPGBeginLoadingScreen`
  (if (not (`KismetSystemLibrary.IsDedicatedServer`))
    (`WidgetLoadingManagerObject.ShowLoadingWidget` (`self.GetWidgetLoadingManagerObject`) (`self.LoadingWidgetSubClass`) 99)))

(event `self.RPGEndLoadingScreen`
  (if (not (`KismetSystemLibrary.IsDedicatedServer`))
    (`WidgetLoadingManagerObject.HideLoadingWidget` (`self.GetWidgetLoadingManagerObject`))))

(event `self.HideLoadingDialog`
  (if (not (`KismetSystemLibrary.IsDedicatedServer`))
    (`WidgetLoadingManagerObject.HideLoadingWidget` (`self.GetWidgetLoadingManagerObject`))))