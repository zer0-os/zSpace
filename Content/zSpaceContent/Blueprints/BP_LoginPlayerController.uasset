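; Player controller for the OWS-backed front end, covering pre-login, login, registration and character selection.
; Screens come from data assets matched to screen resolution and are created by a ManageWidgetsResolution object, whose change event refreshes the controller's widget references.
; It lists, creates, removes and connects OWS characters, saving each one's color as cosmetic custom data and applying it to Character meshes in the level.
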(event `self.ReceiveBeginPlay`
  (`|ExecutionSequence`
    (:`then_0`
      (if (or (`KismetSystemLibrary.IsStandalone`) (`self.IsLocalController`))
        (bind _asbp_zspace_game_instance (cast `/Game/zSpaceContent/Blueprints/Game/BP_ZSpaceGameInstance` (`GameplayStatics.GetGameInstance`)))
        (bind _output_get (set `self.GameInstanceRef` _asbp_zspace_game_instance))
        (bind _output_get_2 (set `self.Manage Widgets Resolution` (`ZSpaceGameInstance.GetManageWidgetsResolution` _output_get)))
        (add `ManageWidgetsResolution.OnWidgetChanged` _output_get_2 (`|CreateDelegate` :!event `OnWidgetChanged`))))
    (:`then_1`
      (`KismetSystemLibrary.Delay` 0.2)
      (bind _returnvalue (`|CreateWidget` "/Game/zSpaceContent/UMG/BG_Vidio/WBP_BackgroundVidio.WBP_BackgroundVidio_C" self))
      (`UserWidget.AddToViewport` _returnvalue 0)
      (`self.CreatePreLoginWidget`)
      (bind _returnvalue_2 (`|CreateWidget` "/Game/zSpaceContent/UMG/WBP_LoadingWidget.WBP_LoadingWidget_C"))
      (set `self.LoadingWidget` _returnvalue_2)
      (set `self.bShowMouseCursor` true)
      (bind _asowsgame_instance (cast `OWSGameInstance` (`GameplayStatics.GetGameInstance`)))
      (`OWSGameInstance.HideLoadingScreen` _asowsgame_instance))))

(event `ShowLoginWidget`
  ;[0 0 1] Show Login Widget
  (`ManageWidgetsResolution.CreateWidgetAndAddViewport` (`self.Manage Widgets Resolution`) self (`UIBlueprintFunctionLibrary.GetWidgetSubClassForCurrentScreen` "/Game/zSpaceContent/UMG/DataAsset/DA_Login.DA_Login") (`UIBlueprintFunctionLibrary.GetCurrentScreenResolutionEnum`))
  (`WidgetBlueprintLibrary.SetInputMode_GameAndUIEx` self (`LoginUserWidgetBase.txtEmail` (`self.LoginWidget`))))

(event `HideLoginWdiget`
  (`Widget.RemoveFromParent` (`self.LoginWidget`)))

(event `ShowPreLoginWidget`
  (`ManageWidgetsResolution.CreateWidgetAndAddViewport` (`self.Manage Widgets Resolution`) self (`UIBlueprintFunctionLibrary.GetWidgetSubClassForCurrentScreen` "/Game/zSpaceContent/UMG/DataAsset/DA_PreLogin.DA_PreLogin") (`UIBlueprintFunctionLibrary.GetCurrentScreenResolutionEnum`)))

(event `ShowRegisterWidget`
  ;[0 0 1] Create Register Widget
  (bind _manage_widgets_resolution (`self.Manage Widgets Resolution`)
    (:`then`
      (`ManageWidgetsResolution.CreateWidgetAndAddViewport` _manage_widgets_resolution self (`UIBlueprintFunctionLibrary.GetWidgetSubClassForCurrentScreen` "/Game/zSpaceContent/UMG/DataAsset/DA_Register.DA_Register") (`UIBlueprintFunctionLibrary.GetCurrentScreenResolutionEnum`))
      (`WidgetBlueprintLibrary.SetInputMode_GameAndUIEx` self (`RegisterUserWidgetBase.FirstName` (`self.RegisterWidget`))))
    (:`else`)))

(event `ShowLoadingDialog`
  (`UserWidget.AddToViewport` (`self.LoadingWidget`) 0))

(event `HideLoadingDialog`
  (`Widget.RemoveFromParent` (`self.LoadingWidget`)))

(event `self.NotifyGetAllCharacters`
  (params (UserCharacters :type "Array of UserCharacter Structure (by ref)"))
  ;[0 0 1] Get All Characters
  (bind _output_get (set `self.UserCharacters` UserCharacters))
  (`self.BindOnGetAllCharacters` _output_get)
  (set `self.NumberOfUserCharacters` (`KismetArrayLibrary.Array_Length` _output_get))
  (if (> (`self.NumberOfUserCharacters`) 0)
    (`self.ShowCurrentUserCharacter`))
  (`self.RefreshCharacterSelection`)
  (`self.RefreshColor`))

(event `ShowSelectCharacterWidget`
  (`ManageWidgetsResolution.CreateWidgetAndAddViewport` (`self.Manage Widgets Resolution`) self (`UIBlueprintFunctionLibrary.GetWidgetSubClassForCurrentScreen` "/Game/zSpaceContent/UMG/DataAsset/DA_SelectCharacter.DA_SelectCharacter") (`UIBlueprintFunctionLibrary.GetCurrentScreenResolutionEnum`))
  (if (`KismetStringLibrary.NotEqual_StrStr` (`self.UserSessionGUID`))
    (`self.GetAllCharacters` (`self.UserSessionGUID`))
    (else
      (`KismetSystemLibrary.PrintString` "UserSessionGUID is empty!"))))

(event `HideSelectCharacterWidget`
  (`Widget.RemoveFromParent` (`self.SelectCharacterRef`)))

(event `self.ErrorGetAllCharacters`
  (params (ErrorMsg :type String))
  (`KismetSystemLibrary.PrintString` ErrorMsg))

(event `self.NotifyCreateCharacter`
  (params (CreateCharacterData :type "CreateCharacter Structure (by ref)"))
  (`SelectCharacterUserWidget.HideCreateNewCharacterWidget` (`self.SelectCharacterRef`))
  (`self.AddCharacterToList` (`.CharacterName` (break `CreateCharacter` CreateCharacterData)) (`self.UserCharacters`))
  (`self.ShowCurrentUserCharacter`)
  (`self.RefreshCharacterSelection`)
  (`self.RefreshColor`))

(event `self.ErrorCreateCharacter`
  (params (ErrorMsg :type String))
  (`KismetSystemLibrary.PrintString` ErrorMsg))

(event `ConnectWithSelectedCharacter`
  (`self.ShowLoadingDialog`)
  (bind _output_get (set `self.SelectedCharacterName` (`.CharacterName` (break `UserCharacter` (`|GetArrayItem` (`self.UserCharacters`) (`self.CurrentlySelectedCharacterIndex`))))))
  (`self.SetSelectedCharacterAndConnectToLastZone` (`self.UserSessionGUID`) _output_get))

(event `Update Character Color`
  (params (Color :type String))
  (bind _output_get (set `self.SelectedCharacterName` (`.CharacterName` (break `UserCharacter` (`|GetArrayItem` (`self.UserCharacters`) (`self.CurrentlySelectedCharacterIndex`))))))
  (if (`KismetStringLibrary.NotEqual_StrStr` _output_get)
    (`self.AddOrUpdateCosmeticCustomCharacterData` (`self.UserSessionGUID`) (`self.SelectedCharacterName`) "CharacterColor" Color)
    (set `self.CharacterColor` Color)
    (`self.RefreshColor`)
    (else
      (`KismetSystemLibrary.PrintString` "Selected Character Name is NULL!"))))

(event `GetCosmeticData`
  (params (CharacterName :type String))
  (`self.GetCosmeticCustomCharacterData` (`self.UserSessionGUID`) CharacterName))

(event `self.NotifyGetCosmeticCustomCharacterData`
  (params (CustomCharacterData :type "Array of CustomCharacterDataStruct Structure (by ref)"))
  (for _array_element CustomCharacterData
    (bind (_customfieldname _fieldvalue) (break `CustomCharacterDataStruct` _array_element))
    (if (`KismetStringLibrary.EqualEqual_StrStr` _customfieldname "CharacterColor")
      (set `self.CharacterColor` _fieldvalue)
      (break)))
  (`self.RefreshColor`)
  (bind _outactors (`GameplayStatics.GetAllActorsOfClass` "/Script/Engine.Character"))
  (for _array_element_2 _outactors
    (`self.SetActorHiddenInGame` _array_element_2 false)))

(event `RemoveACharacter`
  (bind _output_get (set `self.SelectedCharacterName` (`.CharacterName` (break `UserCharacter` (`|GetArrayItem` (`self.UserCharacters`) (`self.CurrentlySelectedCharacterIndex`))))))
  (if (`KismetStringLibrary.NotEqual_StrStr` _output_get)
    (`KismetArrayLibrary.Array_Remove` (`self.UserCharacters`) (`self.CurrentlySelectedCharacterIndex`))
    (`/Engine/EditorBlueprintResources/StandardMacros.DecrementInt` (`self.NumberOfUserCharacters`)
      (:`  `
        (`self.RemoveCharacter` (`self.UserSessionGUID`) (`self.SelectedCharacterName`))
        (`self.DecrementCurrentCharacter`)
        (`self.ShowCurrentUserCharacter`)))
    (else
      (`KismetSystemLibrary.PrintString` "Selected Character Name is NULL!"))))

(fn `AddCharacterToList`
  (params (CharacterName :type String) (UserCharacterList :type "Array of UserCharacter Structure (by ref)"))
  (bind ((`UserCharacter` _usercharacter)) (make `UserCharacter` :`CharacterName` CharacterName))
  (bind ((`CharacterName` _charactername) (`Level` _level)) (break `UserCharacter` _usercharacter))
  (`KismetArrayLibrary.Array_Add` UserCharacterList _usercharacter)
  (bind _result (`/Engine/EditorBlueprintResources/StandardMacros.IncrementInt` (`self.NumberOfUserCharacters`))
    (:`  `
      (set `self.CurrentlySelectedCharacterIndex` (- _result 1))
      (`SelectCharacterBoxUserWidget.SetupWidget` (`SelectCharacterUserWidget.SelectedCharacterBoxUserWidget` (`self.SelectCharacterRef`)) (make `CharacterSelectBoxInfo` _charactername (`KismetStringLibrary.Conv_IntToString` _level))))))

(fn `CreatePreLoginWidget`
  (bind _manage_widgets_resolution (`self.Manage Widgets Resolution`)
    (:`then`
      (`ManageWidgetsResolution.CreateWidgetAndAddViewport` _manage_widgets_resolution self (`UIBlueprintFunctionLibrary.GetWidgetSubClassForCurrentScreen` "/Game/zSpaceContent/UMG/DataAsset/DA_PreLogin.DA_PreLogin") (`UIBlueprintFunctionLibrary.GetCurrentScreenResolutionEnum`))
      (`WidgetBlueprintLibrary.SetInputMode_GameAndUIEx` self null))
    (:`else`)))

(fn `DecrementCurrentCharacter`
  (if (== (`self.CurrentlySelectedCharacterIndex`) 0)
    (set `self.CurrentlySelectedCharacterIndex` (- (`self.NumberOfUserCharacters`) 1))
    (else
      (set `self.CurrentlySelectedCharacterIndex` (- (`self.CurrentlySelectedCharacterIndex`) 1)))))

(fn `IncrementCurrentCharacter`
  (if (== (`self.CurrentlySelectedCharacterIndex`) (- (`self.NumberOfUserCharacters`) 1))
    (set `self.CurrentlySelectedCharacterIndex` 0)
    (else
      (set `self.CurrentlySelectedCharacterIndex` (+ (`self.CurrentlySelectedCharacterIndex`) 1)))))

(fn `OnWidgetChanged`
  (params (Widget :type "UserWidget Object Reference") (WidgetType :type "EWidgetType Enum" :default "PreLogin"))
  (bind _widget (`local.Widget`))
  (switch `EWidgetType` WidgetType
    (:`PreLogin`
      (`self.SetPreLoginWidget` _widget))
    (:`Login`
      (`self.SetLoginWidget` _widget))
    (:`Register`
      (`self.SetRegisterWidget` _widget))
    (:`SelectCharacter`
      (bind _asselect_character_user_widget (cast `SelectCharacterUserWidget` _widget))
      (set `self.SelectCharacterRef` _asselect_character_user_widget))))

(fn `RefreshCharacterSelection`
  (locals (SelectCharacterSwitcher :type "WidgetSwitcher Object Reference"))
  (bind _selectcharacterswitcher (`local.SelectCharacterSwitcher`))
  (bind _selectcharacterswitcher_2 (`local.SelectCharacterSwitcher`))
  (bind _selectcharacterswitcher_3 (`local.SelectCharacterSwitcher`))
  (set `local.SelectCharacterSwitcher` (`SelectCharacterBoxUserWidget.WidgetSwitcherDoneEditMode` (`SelectCharacterUserWidget.SelectedCharacterBoxUserWidget` (`self.SelectCharacterRef`))))
  (`|ExecutionSequence`
    (:`then_0`
      (if (> (`KismetArrayLibrary.Array_Length` (`self.UserCharacters`)) 0)
        (`Widget.SetVisibility` _selectcharacterswitcher_2 "Visible")
        (else
          (`Widget.SetVisibility` _selectcharacterswitcher_2 "Hidden"))))
    (:`then_1`
      (if (> (`KismetArrayLibrary.Array_Length` (`self.UserCharacters`)) (`self.CurrentlySelectedCharacterIndex`))
        (`Widget.SetVisibility` _selectcharacterswitcher_3 "Visible")
        (else
          (`Widget.SetVisibility` _selectcharacterswitcher_3 "Hidden"))))
    (:`then_2`
      (if (> (`KismetArrayLibrary.Array_Length` (`self.UserCharacters`)) 0)
        (`Widget.SetVisibility` _selectcharacterswitcher "Visible")
        (else
          (`Widget.SetVisibility` _selectcharacterswitcher "Hidden"))))))

(fn `RefreshColor`
  (bind (_r _g _b) (break `LinearColor` (`self.CharacterLinearColor`)))
  (if (`KismetStringLibrary.EqualEqual_StrStr` (`self.CharacterColor`) "Red")
    (set `self.CharacterLinearColor` (struct :`R` 1.0 :`A` 1.0))
    (elif (`KismetStringLibrary.EqualEqual_StrStr` (`self.CharacterColor`) "Green")
      (set `self.CharacterLinearColor` (struct :`G` 1.0 :`A` 1.0))
      (elif (`KismetStringLibrary.EqualEqual_StrStr` (`self.CharacterColor`) "Blue")
        (set `self.CharacterLinearColor` (struct :`B` 1.0 :`A` 1.0))
        (else
          (set `self.CharacterLinearColor` (struct :`R` 1.0 :`G` 1.0 :`B` 1.0 :`A` 1.0))))))
  (bind _outactors (`GameplayStatics.GetAllActorsOfClass` "/Script/Engine.Character"))
  (for _array_element _outactors
    (`MeshComponent.SetVectorParameterValueOnMaterials` (`Character.Mesh` _array_element) "BodyColor" (`KismetMathLibrary.MakeVector` _r _g _b))))

(fn `SetLoginWidget`
  (params (Object :type "UserWidget Object Reference"))
  (bind _aswbp_login_base (cast `/Game/zSpaceContent/UMG/Login/WBP_LoginBase` Object))
  (set `self.LoginWidget` _aswbp_login_base))

(fn `SetPreLoginWidget`
  (params (Object :type "UserWidget Object Reference"))
  (bind _aswbp_pre_login_base (cast `/Game/zSpaceContent/UMG/PreLogin/WBP_PreLoginBase` Object))
  (set `self.PreLoginWidget` _aswbp_pre_login_base))

(fn `SetRegisterWidget`
  (params (Object :type "UserWidget Object Reference"))
  (bind _asregister_user_widget_base (cast `RegisterUserWidgetBase` Object))
  (set `self.RegisterWidget` _asregister_user_widget_base))

(fn `ShowCurrentUserCharacter`
  (bind ((`CharacterName` _charactername) (`Level` _level)) (break `UserCharacter` (`|GetArrayItem` (`self.UserCharacters`) (`self.CurrentlySelectedCharacterIndex`))))
  (bind _selectcharacterref (`self.SelectCharacterRef`)
    (:`then`
      (`SelectCharacterUserWidget.CreateCharacterSelectBox` _selectcharacterref (make `CharacterSelectBoxInfo` _charactername (`KismetStringLibrary.Conv_IntToString` _level)))
      (`self.GetCosmeticData` _charactername))
    (:`else`)))

(fn `UserConstructionScript`)