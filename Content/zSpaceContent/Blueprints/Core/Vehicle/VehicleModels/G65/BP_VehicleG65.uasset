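; BP_VehicleG65 is the G65 vehicle Blueprint, a thin child that defers to its parent class for construction and BeginPlay.
; On BeginPlay, only the non-authority (Remote) side opens the Wilder World trailer media source on a MediaPlayer and plays it, provided the player is valid.
; Overlap and Tick events are disabled stubs.
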(event `self.ReceiveBeginPlay`
  (`parent.ReceiveBeginPlay`)
  (`/Engine/EditorBlueprintResources/ActorMacros.Switch Has Authority`
    (:`Remote`
      (bind _mediaplayer (`self.MediaPlayer`)
        (:`then`
          (`MediaPlayer.OpenSource` _mediaplayer "/Game/zSpaceContent/Blueprints/Core/Vehicle/VehicleModels/G65/UI/VideoPlayer/MSF_WilderWorldTrailer.MSF_WilderWorldTrailer")
          (`MediaPlayer.Play` _mediaplayer))
        (:`else`)))))

(fn `UserConstructionScript`
  (`parent.UserConstructionScript`))