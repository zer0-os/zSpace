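; BP_EtherlinkerGameMode is a game mode Blueprint that prints the results of backend-style queries for global data, world time and zone instances.
; Notify and error events print the returned values, including each running zone instance's name, port and status.
; A global data add or update also triggers a world time request, while BeginPlay, Tick and the construction script are empty.
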(event `self.ReceiveBeginPlay`)

(event `self.NotifyAddOrUpdateGlobalDataItem`
  (`KismetSystemLibrary.PrintString` "Added Global Data")
  (`self.GetCurrentWorldTime`))

(event `self.NotifyGetCurrentWorldTime`
  (params (CurrentWorldTime :type "Float (single-precision)"))
  (`KismetSystemLibrary.PrintString` (`KismetStringLibrary.Concat_StrStr` "Current Game World Time: " (`KismetStringLibrary.Conv_DoubleToString` CurrentWorldTime))))

(event `self.ErrorGetCurrentWorldTime`
  (params (ErrorMsg :type String))
  (`KismetSystemLibrary.PrintString` ErrorMsg))

(event `self.NotifyGetGlobalDataItem`
  (params (GlobalDataKey :type String))
  (`KismetSystemLibrary.PrintString` (`KismetStringLibrary.Concat_StrStr` "Global Data Item: " GlobalDataKey)))

(event `self.NotifyGetZoneInstancesForZone`
  (params (ZoneInstances :type "Array of ZoneInstanceStruct Structure (by ref)"))
  (`KismetSystemLibrary.PrintString` "List of running Game Instances:")
  (for _array_element ZoneInstances
    (bind (_mapinstanceid _port _status _zonename) (break `ZoneInstanceStruct` _array_element))
    (`KismetSystemLibrary.PrintString` (`KismetStringLibrary.Concat_StrStr` _zonename " - Port: " (`KismetStringLibrary.Conv_IntToString` _port) " - Status: " (`KismetStringLibrary.Conv_IntToString` _status)))))

(fn `UserConstructionScript`)