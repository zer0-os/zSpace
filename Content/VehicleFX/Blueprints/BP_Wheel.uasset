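; BP_Wheel is a vehicle wheel Blueprint that exposes adjustable dirtiness and wetness on the wheel's materials.
; Its construction script creates a dynamic material instance for each material slot on the Wheel component and adds it to the Materials array.
; It then pushes the Dirtiness and Wetness variables into every instance as scalar parameters.
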(fn `UserConstructionScript`
  (bind _wheel (`self.Wheel`))
  ;[1 1 1] CreateMaterialsArray
  (for _index (range (`PrimitiveComponent.GetNumMaterials` _wheel))
    (bind _returnvalue (`PrimitiveComponent.CreateDynamicMaterialInstance` _wheel _index null))
    (`KismetArrayLibrary.Array_Add` (`self.Materials`) _returnvalue))
  ;[1 1 1] ApplyDynamicDirtinessAndWetness
  (for _array_element (`self.Materials`)
    (`MaterialInstanceDynamic.SetScalarParameterValue` _array_element "Dirtiness" (`self.Dirtiness`)))
  (for _array_element_2 (`self.Materials`)
    (`MaterialInstanceDynamic.SetScalarParameterValue` _array_element_2 "Wetness" (`self.Wetness`))))