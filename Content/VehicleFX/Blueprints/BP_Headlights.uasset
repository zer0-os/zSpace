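; BP_Headlights is a vehicle headlight Blueprint that switches between full-beam and dipped light cones.
; DipLights and FullBeams show one cone and hide the other, propagating to child components, without updating the Dipped flag.
; ToggleLights swaps the cones based on Dipped and flips that flag.
; The construction script shows the dipped cone when Dipped is set, so the starting state applies at construction.
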(event `DipLights`
  ;[1 1 1] DynamicLightControls
  (`SceneComponent.SetVisibility` (`self.LightCone`) false true)
  (`SceneComponent.SetVisibility` (`self.LightCone_Dipped`) true true))

(event `ToggleLights`
  ;[1 1 1] DynamicLightControls
  (if (`self.Dipped`)
    (`SceneComponent.SetVisibility` (`self.LightCone`) true true)
    (`SceneComponent.SetVisibility` (`self.LightCone_Dipped`) false true)
    (set `self.Dipped` false)
    (else
      (`SceneComponent.SetVisibility` (`self.LightCone`) false true)
      (`SceneComponent.SetVisibility` (`self.LightCone_Dipped`) true true)
      (set `self.Dipped` true))))

(event `FullBeams`
  ;[1 1 1] DynamicLightControls
  (`SceneComponent.SetVisibility` (`self.LightCone`) true true)
  (`SceneComponent.SetVisibility` (`self.LightCone_Dipped`) false true))

(fn `UserConstructionScript`
  ;[1 1 1] SwitchToDipped
  (if (`self.Dipped`)
    (`SceneComponent.SetVisibility` (`self.LightCone`) false true)
    (`SceneComponent.SetVisibility` (`self.LightCone_Dipped`) true true)))