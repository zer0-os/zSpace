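; BP_Exhaust_FX_Preview is a preview actor that shows a vehicle exhaust Niagara effect on a moving static mesh.
; The Construction Script assigns the chosen Niagara template and sets its initial User.Intensity.
; On BeginPlay, a timeline slides the mesh along world X from its start position at a fixed yaw and animates User.Intensity.
; The timeline's Backfire event reactivates the particle with a reset when IsBackfire is enabled.
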(event `self.ReceiveBeginPlay`
  (bind _niagaraparticle (`self.NiagaraParticle`))
  ;[1 1 1] Set Position and Intensity
  (set `self.InitialLocation` (`SceneComponent.K2_GetComponentLocation` (`self.StaticMesh`)))
  (bind (_direction __0_5_1_5 _0_1) (`Timeline|Timeline_0`)
    (:`Update`
      (`SceneComponent.K2_SetWorldLocationAndRotation` (`self.StaticMesh`) (+ (`self.InitialLocation`) (* (1000.0 0.0 0.0) __0_5_1_5)) (`KismetMathLibrary.MakeRotator` 0.0 0.0 -90.0) false false)
      (`ParticleSystemComponent.SetFloatParameter` _niagaraparticle "User.Intensity" _0_1))
    (:`Backfire`
      (if (`self.IsBackfire`)
        (`ActorComponent.Activate` _niagaraparticle true)))))

(fn `UserConstructionScript`
  (bind _niagaraparticle (`self.NiagaraParticle`))
  ;[1 1 1] Initialise Template and Intensity
  (`NiagaraComponent.SetAsset` _niagaraparticle (`self.NiagaraTemplate`))
  (`ParticleSystemComponent.SetFloatParameter` _niagaraparticle "User.Intensity" (`self.Intensity`)))