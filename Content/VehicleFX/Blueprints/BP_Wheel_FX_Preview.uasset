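; Preview actor for vehicle wheel effects, pairing a wheel mesh with a Niagara emitter.
; The construction script creates dynamic materials to apply Dirtiness and Wetness, then assigns the Niagara template and its starting Intensity.
; When PreviewFX is set, a timeline on BeginPlay moves and spins the wheel along world X, keeps the emitter just beneath it, and animates User.Intensity.
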(event `self.ReceiveBeginPlay`
  (bind _niagaraeffect (`self.NiagaraEffect`))
  ;[1 1 1] Move Wheel and Emitter and Update Intensity
  (if (`self.PreviewFX`)
    (set `self.InitialPosition` (`SceneComponent.K2_GetComponentLocation` (`self.Wheel`)))
    (bind (_direction __0_5_1_5 _0_1) (`Timeline|Preview`)
      (:`Update`
        (bind _returnvalue (+ (`self.InitialPosition`) (* (1000.0 0.0 0.0) __0_5_1_5)))
        (`SceneComponent.K2_SetWorldLocationAndRotation` (`self.Wheel`) _returnvalue (`KismetMathLibrary.MakeRotator` (* __0_5_1_5 720.0) 0.0 -90.0) false false)
        (`SceneComponent.K2_SetWorldLocationAndRotation` (`self.NiagaraEffect`) (+ _returnvalue (0.0 0.0 -40.0)) (`KismetMathLibrary.MakeRotator` 0.0 0.0 180.0) false false)
        (`ParticleSystemComponent.SetVectorParameter` _niagaraeffect "User.Intensity" (`KismetMathLibrary.Conv_DoubleToVector` _0_1))
        (`ParticleSystemComponent.SetFloatParameter` _niagaraeffect "User.Intensity" _0_1)))))

(fn `UserConstructionScript`
  (bind _wheel (`self.Wheel`))
  (bind _niagaraeffect (`self.NiagaraEffect`))
  ;[1 1 1] CreateMaterialsArray
  (for _index (range (`PrimitiveComponent.GetNumMaterials` _wheel))
    (bind _returnvalue (`PrimitiveComponent.CreateDynamicMaterialInstance` _wheel _index null "None"))
    (`KismetArrayLibrary.Array_Add` (`self.Materials`) _returnvalue))
  ;[1 1 1] ApplyDynamicDirtinessAndWetness
  (for _array_element (`self.Materials`)
    (`MaterialInstanceDynamic.SetScalarParameterValue` _array_element "Dirtiness" (`self.Dirtiness`)))
  (for _array_element_2 (`self.Materials`)
    (`MaterialInstanceDynamic.SetScalarParameterValue` _array_element_2 "Wetness" (`self.Wetness`)))
  ;[1 1 1] InitialiseEffect
  (`NiagaraComponent.SetAsset` _niagaraeffect (`self.NiagaraTemplate`))
  (`FXSystemComponent.SetFloatParameter` _niagaraeffect "User.Intensity" (`self.Intensity`)))